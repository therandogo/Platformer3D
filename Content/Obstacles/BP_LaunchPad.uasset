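; BP_LaunchPad is a lockable obstacle pad that launches the third-person character straight upward.
; When its box is overlapped while unlocked, it plays a sound and calls LaunchCharacter with vertical JumpSpeed, overriding only Z velocity.
; Each Turnedon event increments an unlock counter, and the pad unlocks once the count reaches RequiredUnlockTimes, so several activations can be required.
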(event OnComponentBeginOverlap(Box)
  (params (OverlappedComponent :type Primitive%20Component%20Object%20Reference) (OtherActor :type Actor%20Object%20Reference) (OtherComp :type Primitive%20Component%20Object%20Reference) (OtherBodyIndex :type Integer) (bFromSweep :type Boolean) (SweepResult :type Hit%20Result%20Structure%20%28by%20ref%29))
  (if (not (Variables|Default|GetIsLocked))
    (bind _asbp_third_person_character (Utilities|Casting|CastToBP_ThirdPersonCharacter OtherActor))
    (Audio|PlaySoundatLocation "/Engine/VREditor/Sounds/UI/Floating_UI_Open-001.Floating_UI_Open-001" (Transformation|GetActorLocation) "0, 0, 0" 1.0 1.0 0.0 0 0 0 0)
    (Character|LaunchCharacter _asbp_third_person_character (* "0.000000,0.000000,1.000000" (Variables|Default|GetJumpSpeed)) false true)))

(event EventTurnedon
  (bind _unlocktimes (Variables|Default|GetUnlockTimes))
  (Math|Integer|IncrementInt _unlocktimes
    (:%20%20
      (if (>= _unlocktimes (Variables|Default|GetRequiredUnlockTimes))
        (Variables|Default|SetIsLocked false)))))

(fn ConstructionScript)