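; BP_HeadSwitch is a one-way obstacle switch that changes color when hit and signals a linked actor to unlock.
; CollisionOccured, while the switch is still off, plays a timeline at a configurable rate that blends a dynamic material's color from initial to final.
; Each timeline update also sends TurnedOnMessage to ActorToUnlock and latches the switch on, so the message repeats throughout the blend.
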(event EventCollisionOccured
  (if (not (Variables|Default|GetSwitchState))
    (Components|Timeline|SetPlayRate (Variables|Default|GetColorLerp) (/ 1.0 (Variables|Default|GetLerpRate)))
    (bind _newtrack_0 (Timeline|ColorLerp PlayFromStart)
      (:Update
        (Rendering|Material|SetVectorParameterValue (Variables|Default|GetMaterialInstance) "Color" (Math|Color|Lerp(LinearColor) (Variables|Default|GetInitialColor) (Variables|Default|GetFinalColor) _newtrack_0) :!class /Script/Engine.MaterialInstanceDynamic)
        (Class|BPIHeadSwitchTurnon|Turnedon(Message) (Variables|Default|GetActorToUnlock))
        (Variables|Default|SetSwitchState true)))))

(event EventBeginPlay
  (bind _returnvalue (Rendering|Material|CreateDynamicMaterialInstance (Variables|Default|GetStaticMesh) 0 "/Game/Materials/MI_HeadSwitch.MI_HeadSwitch" "None" :!class /Script/Engine.PrimitiveComponent))
  (bind _output_get (Variables|Default|SetMaterialInstance _returnvalue))
  (Rendering|Material|SetVectorParameterValue _output_get "Color" (Variables|Default|GetInitialColor) :!class /Script/Engine.MaterialInstanceDynamic))

(fn ConstructionScript)