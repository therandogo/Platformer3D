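; BP_SwingingObstacle is a pendulum hazard that swings back and forth and punishes the third-person character on contact.
; A timeline started on BeginPlay lerps the static mesh's pitch between two mirrored angles, alternating forward and reverse playback to loop endlessly.
; When the character begins overlapping the box, it is launched upward and sent OnDeathMessage.
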(event OnComponentBeginOverlap(Box)
  (params (OverlappedComponent :type Primitive%20Component%20Object%20Reference) (OtherActor :type Actor%20Object%20Reference) (OtherComp :type Primitive%20Component%20Object%20Reference) (OtherBodyIndex :type Integer) (bFromSweep :type Boolean) (SweepResult :type Hit%20Result%20Structure%20%28by%20ref%29))
  (bind _asbp_third_person_character (Utilities|Casting|CastToBP_ThirdPersonCharacter OtherActor))
  (Character|LaunchCharacter _asbp_third_person_character (* "0.000000,0.000000,1.000000" 5e+02) false false)
  (Class|BPIDeath|OnDeath(Message) OtherActor))

(event EventBeginPlay
  (bind (_direction _newtrack_0) (Timeline|Pendulum PlayFromStart)
    (:Update
      (Transformation|SetRelativeRotation (Variables|Default|GetStaticMesh) (Math|Rotator|Lerp(Rotator) "-60.000000,0.000000,0.000000" "60.000000,0.000000,0.000000" _newtrack_0) false false))
    (:Finished
      (if (Utilities|Enum|Equal(Enum) _direction "Forward")
        (Timeline|Pendulum Reverse)
        (else
          (Timeline|Pendulum PlayFromStart))))))

(fn ConstructionScript)